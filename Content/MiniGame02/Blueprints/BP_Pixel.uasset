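; BP_Pixel is a cell in a minigame fire-spread simulation that goes from normal to burning to burned.
; OnFire and Burned actor tags drive its state, and Tick applies the matching plane material.
; When burning, from BeginPlay or FireSpread, it waits, then tags overlapping unburned pixels OnFire and calls their FireSpread, chaining the fire outward.
; After a longer delay it swaps its own tag to Burned.
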(event `self.ReceiveTick`
  (params (DeltaSeconds :type "Float (single-precision)"))
  (bind _plane (`self.Plane`))
  (switch `int` (`self.State`)
    (:`0`
      (`PrimitiveComponent.SetMaterial` _plane 0 "/Game/Materials/M_Pixel.M_Pixel")
      (if (`self.ActorHasTag` "OnFire")
        (set `self.State` 1)
        (elif (`self.ActorHasTag` "Burned")
          (set `self.State` 2))))
    (:`1`
      (`PrimitiveComponent.SetMaterial` _plane 0 "/Game/Materials/M_Pixel_OnFire.M_Pixel_OnFire")
      (if (`self.ActorHasTag` "Burned")
        (set `self.State` 2)))
    (:`2`
      (`PrimitiveComponent.SetMaterial` _plane 0 "/Game/Materials/M_Pixel_Burned.M_Pixel_Burned"))))

(event `self.ReceiveBeginPlay`
  (bind _tags (`self.Tags`))
  (if (`self.ActorHasTag` self "OnFire") :!label _label
    (`KismetSystemLibrary.Delay` 4.8)
    (for _array_element (`self.GetOverlappingActors` "BP_Pixel_C")
      (if (not (`self.ActorHasTag` _array_element "Burned"))
        (`KismetArrayLibrary.Array_Add` (`Actor.Tags` _array_element) "OnFire")
        (bind _asbp_pixel (cast `/Game/MiniGame02/Blueprints/BP_Pixel` _array_element))
        (`self.FireSpread` _asbp_pixel)))
    (if (`self.ActorHasTag` "OnFire")
      (`KismetSystemLibrary.Delay` 15.0)
      (`KismetArrayLibrary.Array_RemoveItem` _tags "OnFire")
      (`KismetArrayLibrary.Array_Add` _tags "Burned"))))

(event `FireSpread`
  (goto _label))

(fn `UserConstructionScript`)