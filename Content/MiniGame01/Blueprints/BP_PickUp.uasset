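; BP_PickUp is a trash pickup for MiniGame01 that plays a collection animation on the character's wheelbarrow.
; On overlap it saves the character's speed, moves itself just ahead of the character based on movement direction and raises a Scale flag.
; While flagged, Tick halts the character in its idle flipbook and grows, then shrinks the trash.
; After a short delay it restores movement, moves the trash out of view and resets its scale values.
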(event `self.ReceiveTick`
  (params (DeltaSeconds :type "Float (single-precision)"))
  (if (`self.Scale`)
    (bind _outactors (`GameplayStatics.GetAllActorsOfClass` "/Game/MiniGame01/Blueprints/C_MiniGame01.C_MiniGame01_C"))
    (bind _output (`|GetArrayItem` _outactors))
    ;[1 1 1] charakter bleibt stehn
    (set `/Game/MiniGame01/Blueprints/C_MiniGame01.moveSpeedX` 0.0 _output)
    (set `/Game/MiniGame01/Blueprints/C_MiniGame01.moveSpeedZ` 0.0 _output)
    (`PaperFlipbookComponent.SetFlipbook` (`PaperCharacter.Sprite` _output) "/Game/MiniGame01/Sprites/Character/Idle/FB_C_MiniGame01_Idle.FB_C_MiniGame01_Idle")
    (if (>= (.x (`self.scaleValue`)) (`self.scaleFactor`))
      ;[1 1 1] verkleinert das objekt anschließend
      (set `self.scaleFactor` 0.0)
      (bind _output_get (set `self.scaleValue` (- (`self.scaleValue`) (0.2 0.2 0.0))))
      (`self.K2_AddActorLocalTransform` (`KismetMathLibrary.MakeTransform` (0.0 0.0 0.0) (struct) _output_get))
      (if (<= (.x (`self.scaleValue`)) 0.0)
        (set `self.Scale` false)
        ;[1 1 1] nach kurzer zeit charakter läuft wieder müll objekt wird aus sichtbereich versetzt und ScaleFactor wieder auf 3 gesetzt
        (`KismetSystemLibrary.Delay` 0.4)
        (set `/Game/MiniGame01/Blueprints/C_MiniGame01.moveSpeedX` (`self.saveSpeedX`) _output)
        (set `/Game/MiniGame01/Blueprints/C_MiniGame01.moveSpeedZ` (`self.saveSpeedZ`) _output)
        (`self.K2_SetActorLocation` (`KismetMathLibrary.MakeVector` (`self.pickUpPosX`) 0.0 1000.0))
        (set `self.scaleFactor` 3.0)
        (bind _output_get_2 (set `self.scaleValue` (2.0 2.0 1.0)))
        (`self.K2_AddActorLocalTransform` (`KismetMathLibrary.MakeTransform` (0.0 0.0 0.0) (struct) _output_get_2)))
      (else
        ;[1 1 1] vergrößert das objekt so lange der ScaleFactor eingehalten wird
        (if (not (<= (`self.scaleFactor`) 0.0))
          (bind _output_get_3 (set `self.scaleValue` (+ (`self.scaleValue`) (0.05 0.05 0.0))))
          (`self.K2_AddActorLocalTransform` (`KismetMathLibrary.MakeTransform` (0.0 0.0 0.0) (struct) _output_get_3)))))))

(event `self.ReceiveActorBeginOverlap`
  (params (OtherActor :type "Actor Object Reference"))
  (set `self.pickUpPosX` (.x (`self.K2_GetActorLocation`)))
  (bind _outactors (`GameplayStatics.GetAllActorsOfClass` "/Game/MiniGame01/Blueprints/C_MiniGame01.C_MiniGame01_C"))
  ;[1 1 1] erlaubt dem EVENT TICK das skalieren von den müllobjekten | Müll wird auf schubkarre  mitte verschoben
  (set `self.Scale` true)
  (bind _output (`|GetArrayItem` _outactors))
  (if (>= (`/Game/MiniGame01/Blueprints/C_MiniGame01.moveSpeedX` _output) 0.0)
    (bind _x (.x (`/Game/MiniGame01/Blueprints/C_MiniGame01.characterPos` _output)))
    (bind _y (.y (`/Game/MiniGame01/Blueprints/C_MiniGame01.characterPos` _output)))
    (bind _z (.z (`/Game/MiniGame01/Blueprints/C_MiniGame01.characterPos` _output)))
    (`self.K2_SetActorLocation` (`KismetMathLibrary.MakeVector` (+ _x 60.0) _y _z))
    (else
      (`self.K2_SetActorLocation` (`KismetMathLibrary.MakeVector` (- _x 60.0) _y _z))))
  ;[1 1 1] aktuelle geschwindigkeit in X und Z Richtung wird zwischengespeichert
  (set `self.saveSpeedX` (`/Game/MiniGame01/Blueprints/C_MiniGame01.moveSpeedX` _output))
  (set `self.saveSpeedZ` (`/Game/MiniGame01/Blueprints/C_MiniGame01.moveSpeedZ` _output)))

(fn `UserConstructionScript`)