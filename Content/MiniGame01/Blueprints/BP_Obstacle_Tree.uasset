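; Tree obstacle for MiniGame01 that punishes C_MiniGame01 on overlap with a stun, knockback and loss of collected trash.
; Overlap zeroes move speed and flashes the sprite red via chained delays, while Tick shifts the character along X based on sprite rotation.
; StopCharacterPos is set to X-400, then immediately overwritten with X+400.
; Afterwards, a random pick with fallthrough decrements a metal, plastic or paper counter and destroys a matching pickup.
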(event `self.ReceiveActorBeginOverlap`
  (params (OtherActor :type "Actor Object Reference"))
  (bind _returnvalue (`KismetMathLibrary.RandomIntegerInRange` 1 3))
  (`parent.ReceiveActorBeginOverlap` OtherActor)
  (bind _outactors (`GameplayStatics.GetAllActorsOfClass` "/Game/MiniGame01/Blueprints/C_MiniGame01.C_MiniGame01_C"))
  (bind _output (`|GetArrayItem` _outactors))
  (set `self.saveMoveSpeedX` (`/Game/MiniGame01/Blueprints/C_MiniGame01.moveSpeedX` _output))
  (set `self.saveMoveSpeedZ` (`/Game/MiniGame01/Blueprints/C_MiniGame01.moveSpeedZ` _output))
  (bind _x (.x (`/Game/MiniGame01/Blueprints/C_MiniGame01.characterPos` _output)))
  ;[1 1 1] variablen für rückwurf des characters
  (set `self.stopCharacterPos-` (- _x 400.0))
  (set `self.stopCharacterPos+` (+ _x 400.0))
  (set `self.setAnimation` true)
  (set `/Game/MiniGame01/Blueprints/C_MiniGame01.moveSpeedX` 0.0 _output)
  (set `/Game/MiniGame01/Blueprints/C_MiniGame01.moveSpeedZ` 0.0 _output)
  (bind _sprite (`PaperCharacter.Sprite` _output))
  (set `self.saveSpriteColor` (`PaperFlipbookComponent.SpriteColor` _sprite))
  ;[1 1 1] blinkeffekt des characters
  (`PaperFlipbookComponent.SetSpriteColor` _sprite (struct :`R` 1.0 :`A` 1.0))
  (`KismetSystemLibrary.Delay` 0.2)
  (`PaperFlipbookComponent.SetSpriteColor` _sprite (`self.saveSpriteColor`))
  (`KismetSystemLibrary.Delay` 0.2)
  (`PaperFlipbookComponent.SetSpriteColor` _sprite (struct :`R` 1.0 :`A` 1.0))
  (`KismetSystemLibrary.Delay` 0.2)
  (`PaperFlipbookComponent.SetSpriteColor` _sprite (`self.saveSpriteColor`))
  (`KismetSystemLibrary.Delay` 0.2)
  (`PaperFlipbookComponent.SetSpriteColor` _sprite (struct :`R` 1.0 :`A` 1.0))
  (`KismetSystemLibrary.Delay` 0.2)
  (`PaperFlipbookComponent.SetSpriteColor` _sprite (`self.saveSpriteColor`))
  (`KismetSystemLibrary.Delay` 0.2)
  (`PaperFlipbookComponent.SetSpriteColor` _sprite (struct :`R` 1.0 :`A` 1.0))
  (`KismetSystemLibrary.Delay` 0.2)
  (`PaperFlipbookComponent.SetSpriteColor` _sprite (`self.saveSpriteColor`))
  (`KismetSystemLibrary.Delay` 0.2)
  (`PaperFlipbookComponent.SetSpriteColor` _sprite (struct :`R` 1.0 :`A` 1.0))
  (`KismetSystemLibrary.Delay` 0.2)
  (`PaperFlipbookComponent.SetSpriteColor` _sprite (`self.saveSpriteColor`))
  (`KismetSystemLibrary.Delay` 0.2)
  (set `/Game/MiniGame01/Blueprints/C_MiniGame01.moveSpeedZ` (`self.saveMoveSpeedZ`) _output)
  (set `/Game/MiniGame01/Blueprints/C_MiniGame01.moveSpeedX` (`self.saveMoveSpeedX`) _output)
  (set `self.setAnimation` false)
  ;[1 1 1] verliert den müll von der karre immer eins
  (if (== _returnvalue 1) :!label _label
    (if (> (`/Game/MiniGame01/Blueprints/C_MiniGame01.counterMetal` _output) 0)
      (bind _countermetal (`/Game/MiniGame01/Blueprints/C_MiniGame01.counterMetal` _output))
      (set `/Game/MiniGame01/Blueprints/C_MiniGame01.counterMetal` (- _countermetal 1) _output)
      (bind _outactors_2 (`GameplayStatics.GetAllActorsOfClass` "/Game/MiniGame01/Blueprints/BP_PickUpCollect_Metal.BP_PickUpCollect_Metal_C"))
      (`KismetSystemLibrary.Delay` 1.0)
      (`self.K2_DestroyActor` (`|GetArrayItem` _outactors_2 _countermetal))
      (else
        (if (> (`/Game/MiniGame01/Blueprints/C_MiniGame01.counterPlastic` _output) 0) :!label _label_2
          (bind _counterplastic (`/Game/MiniGame01/Blueprints/C_MiniGame01.counterPlastic` _output))
          (set `/Game/MiniGame01/Blueprints/C_MiniGame01.counterPlastic` (- _counterplastic 1) _output)
          (bind _outactors_3 (`GameplayStatics.GetAllActorsOfClass` "/Game/MiniGame01/Blueprints/BP_PickUpCollect_Plastic.BP_PickUpCollect_Plastic_C"))
          (`KismetSystemLibrary.Delay` 1.0)
          (`self.K2_DestroyActor` (`|GetArrayItem` _outactors_3 _counterplastic))
          (else
            (if (> (`/Game/MiniGame01/Blueprints/C_MiniGame01.counterPaper` _output) 0) :!label _label_3
              (bind _counterpaper (`/Game/MiniGame01/Blueprints/C_MiniGame01.counterPaper` _output))
              (set `/Game/MiniGame01/Blueprints/C_MiniGame01.counterPaper` (- _counterpaper 1) _output)
              (bind _outactors_4 (`GameplayStatics.GetAllActorsOfClass` "/Game/MiniGame01/Blueprints/BP_PickUpCollect_Paper.BP_PickUpCollect_Paper_C"))
              (`KismetSystemLibrary.Delay` 1.0)
              (`self.K2_DestroyActor` (`|GetArrayItem` _outactors_4 _counterpaper)))))))
    (elif (== _returnvalue 2)
      (goto _label_2)
      (elif (== _returnvalue 3)
        (goto _label_3)
        (else
          (goto _label))))))

(event `self.ReceiveTick`
  (params (DeltaSeconds :type "Float (single-precision)"))
  ;[1 1 1] wird nur ausgeführt wenn "setAnimation"
  (if (`self.setAnimation`)
    (bind _output (`|GetArrayItem` (stale `self.ReceiveActorBeginOverlap` _outactors)))
    ;[1 1 1] character wird zurück gestossen bis zu einem bestimmtem wert "stopCharacterPos+,-
    (if (== (`/Game/MiniGame01/Blueprints/C_MiniGame01.rotationSpriteCharacter` _output) 0.0)
      (bind (_characterpos_x _characterpos_y _characterpos_z) (`KismetMathLibrary.BreakVector` (`/Game/MiniGame01/Blueprints/C_MiniGame01.characterPos` _output)))
      (if (>= _characterpos_x (`self.stopCharacterPos-`))
        (set `/Game/MiniGame01/Blueprints/C_MiniGame01.characterPos` (`KismetMathLibrary.MakeVector` (- _characterpos_x 16.0) _characterpos_y _characterpos_z) _output))
      (elif (<= _characterpos_x (`self.stopCharacterPos+`))
        (set `/Game/MiniGame01/Blueprints/C_MiniGame01.characterPos` (`KismetMathLibrary.MakeVector` (+ _characterpos_x 16.0) _characterpos_y _characterpos_z) _output)))))

(fn `UserConstructionScript`
  (`parent.UserConstructionScript`))