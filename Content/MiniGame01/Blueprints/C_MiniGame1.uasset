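; C_MiniGame1 is the MiniGame01 flipbook character, which moves along X automatically while the mouse steers its height.
; BeginPlay stores its position and pauses the game; each Tick adds the X speed and teleport-free, sweep-free sets the location with Y locked to zero.
; Mouse presses store the cursor's visibility-trace hit point, and CharacterMove steps the next Z toward it by a fixed per-frame speed, without delta-time scaling.
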(event `self.ReceiveBeginPlay`
  (`|ExecutionSequence`
    (:`then_0`
      ;[1 1 1] Speichert aktuelle Position vom Charakter
      (set `self.characterPos` (`self.K2_GetActorLocation`))
      (`GameplayStatics.SetGamePaused` true))))

(event `self.ReceiveTick`
  (params (DeltaSeconds :type "Float (single-precision)"))
  (`|ExecutionSequence`
    (:`then_0`
      ;[1 1 1] Bewegt Charakter in X-Richtung
      (set `self.characterPos` (`KismetMathLibrary.MakeVector` (+ (.x (`self.characterPos`)) (`self.moveSpeedX`)) 0.0 (`self.movePosZ`)))
      (`self.K2_SetActorLocation` (`self.characterPos`))
      (`PaperFlipbookComponent.SetFlipbook` (`self.Sprite`) null))
    (:`then_1`
      (`self.CharacterMove`) ; funktion charakter bewegung durch mausklick in z-richtung +-
    )))

(event `InputAction|MouseButton`
  (params (Key :type "Key Structure"))
  (:`Pressed`
    ;[1 1 1] Aktuelle Maus-Position abfragen/speichern
    (set `self.currentMousePos` (`KismetMathLibrary.MakeVector` (.x (`.Location` (`GameplayStatics.BreakHitResult` (`PlayerController.GetHitResultUnderCursorByChannel` (`GameplayStatics.GetPlayerController` 0) "TraceTypeQuery1" true)))) 0.0 (.z (`.Location` (`GameplayStatics.BreakHitResult` (`PlayerController.GetHitResultUnderCursorByChannel` (`GameplayStatics.GetPlayerController` 0) "TraceTypeQuery1" true))))))
    (`/Engine/EditorBlueprintResources/StandardMacros.Do N` 0 :!label _label
      (:`Exit`
        ;[1 1 1] Debug / print aktuelle Maus-Position
        (`KismetSystemLibrary.PrintString` (`KismetStringLibrary.Conv_VectorToString` (`self.currentMousePos`))))))
  (:`Released`
    (goto _label :!via `Reset`)))

(fn `CharacterMove`
  (bind _movespeedz (`self.moveSpeedZ`))
  (bind _z (.z (`self.characterPos`)))
  (bind _z_2 (.z (`self.currentMousePos`)))
  (bind _returnvalue (- _z _movespeedz))
  (bind _returnvalue_2 (+ _z _movespeedz))
  (if (<= _returnvalue_2 _z_2)
    (set `self.movePosZ` _returnvalue_2)
    (elif (>= _returnvalue _z_2)
      (set `self.movePosZ` _returnvalue))))

(fn `UserConstructionScript`)