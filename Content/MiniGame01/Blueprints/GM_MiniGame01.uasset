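; GM_MiniGame01 is the game mode for MiniGame01, running a countdown timer that ends the round.
; Tick feeds a one-second Delay that decrements Seconds and rolls over into Minutes.
; When both reach zero, it prints a time-out message, converts the C_MiniGame01 player character's WasteStatus into a scaled integer Score, resets that status and pauses the game.
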(event `self.ReceiveTick`
  (params (DeltaSeconds :type "Float (single-precision)"))
  ;[1 1 1] Timer für GameOver wenn Zeit abgelaufen ist
  (`KismetSystemLibrary.Delay` 1.0)
  (set `self.seconds` (- (`self.seconds`) 1))
  (if (< (`self.seconds`) 0)
    (set `self.minutes` (- (`self.minutes`) 1))
    (set `self.seconds` 59))
  (if (== (`self.seconds`) 0)
    (if (== (`self.minutes`) 0)
      (`KismetSystemLibrary.PrintString` "time out")
      ;[1 1 1] Setzt Score
      (bind _asc_mini_game_01 (cast `/Game/MiniGame01/Blueprints/C_MiniGame01` (`GameplayStatics.GetPlayerCharacter` 0)))
      (set `self.score` (`KismetMathLibrary.FTrunc` (* (`/Game/MiniGame01/Blueprints/C_MiniGame01.wasteStatus` _asc_mini_game_01) 1000.0)))
      (set `/Game/MiniGame01/Blueprints/C_MiniGame01.wasteStatus` 0.0 _asc_mini_game_01)
      (`GameplayStatics.SetGamePaused` true))))

(fn `UserConstructionScript`)