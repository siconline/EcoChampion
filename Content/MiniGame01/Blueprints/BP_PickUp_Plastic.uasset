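; Plastic trash pickup for MiniGame01 that spawns a collected-plastic actor on overlap, with excess trash meant to fall off the wheelbarrow.
; On BeginPlay it caches the first C_MiniGame01 actor for access to its CounterPlastic.
; Any overlap spawns BP_PickUpCollect_Plastic offset from the pickup, after the parent handler runs.
; If the counter exceeds three, it waits briefly, destroys the collected actor indexed by the counter and decrements it.
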(event `self.ReceiveBeginPlay`
  (`parent.ReceiveBeginPlay`)
  (bind _outactors (`GameplayStatics.GetAllActorsOfClass` "/Game/MiniGame01/Blueprints/C_MiniGame01.C_MiniGame01_C"))
  (set `self.C_MiniGame01_Reference` (`|GetArrayItem` _outactors)))

(event `self.ReceiveActorBeginOverlap`
  (params (OtherActor :type "Actor Object Reference"))
  (bind _c_minigame01_reference (`self.C_MiniGame01_Reference`))
  (`parent.ReceiveActorBeginOverlap` OtherActor)
  ;[1 1 1] wird zu viel muell gesammelt faellt er von der schubkarre
  (`|SpawnActorFromClass` "/Game/MiniGame01/Blueprints/BP_PickUpCollect_Plastic.BP_PickUpCollect_Plastic_C" (`KismetMathLibrary.MakeTransform` (`KismetMathLibrary.MakeVector` (+ (.x (`self.K2_GetActorLocation`)) 100.0) (.y (`self.K2_GetActorLocation`)) (+ (.z (`self.K2_GetActorLocation`)) 100.0))) "Undefined" "OverrideRootScale" null null)
  (if (> (`/Game/MiniGame01/Blueprints/C_MiniGame01.counterPlastic` (`self.C_MiniGame01_Reference`)) 3)
    (`KismetSystemLibrary.Delay` 2.0)
    (bind _outactors (`GameplayStatics.GetAllActorsOfClass` "/Game/MiniGame01/Blueprints/BP_PickUpCollect_Plastic.BP_PickUpCollect_Plastic_C"))
    (`self.K2_DestroyActor` (`|GetArrayItem` _outactors (- (`/Game/MiniGame01/Blueprints/C_MiniGame01.counterPlastic` (`self.C_MiniGame01_Reference`)) 1)))
    (set `/Game/MiniGame01/Blueprints/C_MiniGame01.counterPlastic` (- (`/Game/MiniGame01/Blueprints/C_MiniGame01.counterPlastic` _c_minigame01_reference) 1) _c_minigame01_reference)))

(fn `UserConstructionScript`
  (`parent.UserConstructionScript`))