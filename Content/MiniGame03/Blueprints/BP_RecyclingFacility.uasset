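; Recycling facility actor for MiniGame03 that takes a clicked waste drop and checks whether the item matches the facility's index.
; Tick drives a flag-based sequence: a timeline drops the waste, then per-frame offsets slide it inward.
; A match adds score in GM_MiniGame03, while a mismatch slides back out through a second timeline.
; Overlap negates the character's walk speed and disables the box collision until the item resolves.
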(event `Set Material Facility`
  ;[1 1 1] set material Recycling Facility
  (`PrimitiveComponent.SetMaterial` (`self.StaticMesh`) 0 (`|GetArrayItem` (`self.arrayMaterial`) (`self.index`))))

(event `self.ReceiveBeginPlay`
  ;[1 1 1] start Events
  (`|ExecutionSequence`
    (:`then_0`
      (if true
        (`self.Set Material Facility`)))
    (:`then_1`
      (if true
        (`self.Set Visibility Waste False`)))
    (:`then_2`
      (if true
        (`self.Set Start Position Waste`)))))

(event `Set Material Waste`
  ;[1 1 1] set material Waste --> material index
  (`PrimitiveComponent.SetMaterial` (`self.waste`) 0 (`|GetArrayItem` (`self.arrayMaterialWaste`) (`self.materialWasteIndex`))))

(event `Set Start Position Waste`
  (bind _waste (`self.waste`))
  ;[1 1 1] set start position waste
  (`SceneComponent.K2_SetRelativeLocation` _waste (`KismetMathLibrary.MakeVector` (- (.x (`SceneComponent.RelativeLocation` _waste)) 200.0) (.y (`SceneComponent.RelativeLocation` _waste)) (.z (`SceneComponent.RelativeLocation` _waste))) false false))

(event `Set Visibility Waste False`
  ;[1 1 1] at the begin -- visibility is false
  (bind _output_get (set `self.waste` (`self.waste`)))
  (`SceneComponent.SetVisibility` _output_get false false))

(event `save max walk speed`
  ;[1 1 1] save max walk speed
  (set `self.saveMaxWalkSpeed` (`CharacterMovementComponent.MaxWalkSpeed` (`Character.CharacterMovement` (`GameplayStatics.GetPlayerCharacter` 0)))))

(event `Set Wrong or Right Item`
  ;[1 1 1] set wrong or right item
  (if (== (`self.index`) (`self.materialWasteIndex`))
    (set `self.checkItem` true)
    (else
      (set `self.checkItem` false))))

(event `self.ReceiveTick`
  (params (DeltaSeconds :type "Float (single-precision)"))
  ;[1 1 1] start Events
  (`|ExecutionSequence`
    (:`then_0`
      (if true
        (`self.Set Material Waste`)))
    (:`then_1`
      (if true
        (`self.Set Wrong or Right Item`)))
    (:`then_2`
      (if true
        (`self.Animation dropping Item`)))
    (:`then_3`
      (if true
        (`self.Animation wrong Item`)))))

(event `Animation dropping Item`
  (bind _waste (`self.waste`))
  (bind _x (.x (`SceneComponent.RelativeLocation` _waste)))
  ;[1 1 1] animation dropping item
  (if (not (`self.startMove`))
    (if (`self.startAnimation`)
      ;;[1 1 1] set visibility true
      (bind _output_get (set `self.waste` (`self.waste`)))
      (`SceneComponent.SetVisibility` _output_get true false)
      ;;[1 1 1] play animation drop waste
      (bind (_direction _animation _scale) (`Timeline|Animation_Waste` :!label _label)
        (:`Update`
          (`SceneComponent.K2_SetRelativeLocation` (`self.waste`) _animation false false)
          (`SceneComponent.SetRelativeScale3D` (`self.waste`) _scale))
        (:`Finished`
          (set `self.startMove` true)
          (set `self.startAnimation` false))))
    (elif (and (not (`self.wrongItem`)) (`self.startMove`))
      ;;[1 1 1] animation move waste
      (`SceneComponent.K2_SetRelativeLocation` _waste (`KismetMathLibrary.MakeVector` (+ _x 1.0) (.y (`SceneComponent.RelativeLocation` _waste)) (.z (`SceneComponent.RelativeLocation` _waste))) false false)
      (if (>= _x 0.0)
        ;;[1 1 1] ! > > manipulate checkItem < < ! WRONG or RIGHT ITEM
        (if (`self.checkItem`)
          (set `self.startMove` false)
          ;;[1 1 1] set visibility false
          (bind _output_get_2 (set `self.waste` (`self.waste`)))
          (`SceneComponent.SetVisibility` _output_get_2 false false)
          (`PrimitiveComponent.SetCollisionEnabled` (`self.Box`) "QueryAndPhysics")
          (`self.resetAnimationWaste`) ; reset animation
          (`self.Set Score`)
          (else
            (set `self.wrongItem` true)))))))

(event `self.ReceiveActorOnClicked`
  (params (ButtonPressed :type "Key Structure"))
  ;[1 1 1] start Events
  (`|ExecutionSequence`
    (:`then_0`
      (if true
        (`self.Start Animation`)))))

(event `resetAnimationWaste`
  ;[1 1 1] animation dropping item
  ;;[1 1 1] play animation drop waste
  (goto _label :!via `SetNewTime`))

(event `self.ReceiveActorBeginOverlap`
  (params (OtherActor :type "Actor Object Reference"))
  ;[1 1 1] start Events
  (`|ExecutionSequence`
    (:`then_0`
      (if true
        (`self.save max walk speed`)))
    (:`then_1`
      (if true
        (`self.Character Move Stop` OtherActor)))))

(event `Set Score`
  ;[1 1 1] set score
  (`/Engine/EditorBlueprintResources/StandardMacros.IsValid` "/Game/MiniGame03/Blueprints/GM_MiniGame03.GM_MiniGame03"
    (:`Is Valid`
      (bind _asgm_mini_game_03 (cast `/Game/MiniGame03/Blueprints/GM_MiniGame03` (`GameplayStatics.GetGameMode`)))
      (set `/Game/MiniGame03/Blueprints/GM_MiniGame03.score` (+ (`/Game/MiniGame03/Blueprints/GM_MiniGame03.score` _asgm_mini_game_03) 1) _asgm_mini_game_03))
    (:`Is Not Valid`
      (`KismetSystemLibrary.PrintString` "missing gamemode GM_MiniGame03"))))

(event `Animation wrong Item`
  (bind _waste (`self.waste`))
  (bind _x (.x (`SceneComponent.RelativeLocation` _waste)))
  ;[1 1 1] animation wrong item
  (if (`self.wrongItem`)
    (`SceneComponent.K2_SetRelativeLocation` _waste (`KismetMathLibrary.MakeVector` (- _x 1.0) (.y (`SceneComponent.RelativeLocation` _waste)) (.z (`SceneComponent.RelativeLocation` _waste))) false false)
    (if (<= _x -200.0)
      (bind (_direction _animation) (`Timeline|animationWrongWaste` :!label _label_2)
        (:`Update`
          (`SceneComponent.K2_SetRelativeLocation` (`self.waste`) _animation false false))
        (:`Finished`
          (set `self.wrongItem` false)
          (set `self.startMove` false)
          ;;[1 1 1] set visibility false
          (bind _output_get (set `self.waste` (`self.waste`)))
          (`SceneComponent.SetVisibility` _output_get false false)
          (`PrimitiveComponent.SetCollisionEnabled` (`self.Box`) "QueryAndPhysics")
          ;;[1 1 1] reset animations
          (`self.resetAnimationWrongWaste`)
          (`self.resetAnimationWaste`))))))

(event `resetAnimationWrongWaste`
  ;[1 1 1] animation wrong item
  (goto _label_2 :!via `SetNewTime`))

(event `Character Move Stop`
  (params (`Other Actor` :type "Actor Object Reference"))
  ;[1 1 1] character stop moving -- collision box disabled
  (bind _ascharacter (cast `Character` `Other Actor`))
  (set `CharacterMovementComponent.MaxWalkSpeed` (* (`self.saveMaxWalkSpeed`) -1.0) (`Character.CharacterMovement` _ascharacter))
  (`PrimitiveComponent.SetCollisionEnabled` (`self.Box`) "NoCollision"))

(event `Start Animation`
  ;[1 1 1] start animation
  (if (`self.clickable`)
    (set `self.startAnimation` true)
    (set `self.clickable` false)))

(fn `UserConstructionScript`)