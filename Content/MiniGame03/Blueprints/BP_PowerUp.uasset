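; Pickup for MiniGame03 that is either an eco boost or a wheelbarrow tool upgrade, with a matching plane material.
; On player overlap it calls the matching carry function on C_MiniGame03; any overlapping Character also saves its walk speed and starts the scale animation.
; Tick snaps the pickup to the player and runs a grow-then-shrink effect, then destroys it, restores the player's saved speed and plays a sound.
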(event `Set Type Boost`
  ;[1 1 1] Set Material
  (set `self.isBoost` true)
  (`PrimitiveComponent.SetMaterial` (`self.Plane`) 0 "/Game/Materials/M_EcoBoost.M_EcoBoost"))

(event `Set Type Upgrade`
  ;[1 1 1] Set Material
  (set `self.isBoost` false)
  (`PrimitiveComponent.SetMaterial` (`self.Plane`) 0 "/Game/Materials/M_EcoTool.M_EcoTool"))

(event `self.ReceiveBeginPlay`
  ;[1 1 1] Start events
)

(event `self.ReceiveActorBeginOverlap`
  (params (OtherActor :type "Actor Object Reference"))
  ;[1 1 1] Start events
  (`|ExecutionSequence`
    (:`then_0`
      (if true
        ;[1 1 1] On Overlap
        (if (== (`GameplayStatics.GetPlayerCharacter` 0) OtherActor)
          (`|ExecutionSequence`
            (:`then_0`
              (if (`self.isBoost`)
                (bind _outactors (`GameplayStatics.GetAllActorsOfClass` "/Game/MiniGame03/Blueprints/C_MiniGame03.C_MiniGame03_C"))
                (bind _asc_mini_game_03 (cast `/Game/MiniGame03/Blueprints/C_MiniGame03` (`|GetArrayItem` _outactors)))
                (`/Game/MiniGame03/Blueprints/C_MiniGame03.carryBoost` _asc_mini_game_03)
                (else
                  (bind _outactors_2 (`GameplayStatics.GetAllActorsOfClass` "/Game/MiniGame03/Blueprints/C_MiniGame03.C_MiniGame03_C"))
                  (bind _asc_mini_game_03_2 (cast `/Game/MiniGame03/Blueprints/C_MiniGame03` (`|GetArrayItem` _outactors_2)))
                  (`/Game/MiniGame03/Blueprints/C_MiniGame03.carryWheelbarrowUpgrade` _asc_mini_game_03_2))))))))
    (:`then_1`
      (if true
        (`self.Save MaxWalkSpeed` OtherActor)))
    (:`then_2`
      (if true
        (`self.Set Value for animation scale` OtherActor)))))

(event `Play Animation Scale`
  ;[1 1 1] set boolean SCALE --> true -- begin actor grow and shrink
  (if (`self.scale`)
    (`self.K2_SetActorLocation` (`self.K2_GetActorLocation` (`GameplayStatics.GetPlayerCharacter` 0)))
    (if (>= (.x (`self.scaleValue`)) (`self.scaleFactor`))
      (set `self.scaleFactor` 0.0)
      (bind _output_get (set `self.scaleValue` (- (`self.scaleValue`) (0.2 0.2 0.0))))
      (`self.K2_AddActorLocalTransform` (`KismetMathLibrary.MakeTransform` (0.0 0.0 0.0) (struct) _output_get))
      (if (<= (.x (`self.scaleValue`)) 1.0)
        (`self.Destroy Actor`))
      (elif (not (<= (`self.scaleFactor`) 0.0))
        (bind _output_get_2 (set `self.scaleValue` (+ (`self.scaleValue`) (0.05 0.05 0.0))))
        (`self.K2_AddActorLocalTransform` (`KismetMathLibrary.MakeTransform` (0.0 0.0 0.0) (struct) _output_get_2))))))

(event `self.ReceiveTick`
  (params (DeltaSeconds :type "Float (single-precision)"))
  ;[1 1 1] Start events
  (`|ExecutionSequence`
    (:`then_0`
      (if true
        (`self.Play Animation Scale`)))
    (:`then_1`
      (if true
        (`self.check Direction Character`)))))

(event `Destroy Actor`
  ;[1 1 1] destroy actor -- reset charactermovement speed -- reset boolean SCALE
  (`self.K2_DestroyActor`)
  (set `CharacterMovementComponent.MaxWalkSpeed` (`self.saveMaxWalkSpeed`) (`Character.CharacterMovement` (`GameplayStatics.GetPlayerCharacter` 0)))
  (set `self.scale` false)
  (`self.reset`)
  (`GameplayStatics.PlaySound2D` "/Game/Sounds/S_blob.S_Blob") ; PickUp Sound
)

(event `Save MaxWalkSpeed`
  (params (`Other Actor` :type "Actor Object Reference"))
  ;[1 1 1] save MaxWalkSpeed and diable input
  (bind _ascharacter (cast `Character` `Other Actor`))
  (`/Engine/EditorBlueprintResources/StandardMacros.Do N` 1 :!label _label
    (:`Exit`
      (set `self.saveMaxWalkSpeed` (`CharacterMovementComponent.MaxWalkSpeed` (`Character.CharacterMovement` _ascharacter))))))

(event `reset`
  ;[1 1 1] save MaxWalkSpeed and diable input
  (goto _label :!via `Reset`))

(event `Set Value for animation scale`
  (params (`Other Actor` :type "Actor Object Reference"))
  ;[1 1 1] set value for animation scale
  (cast `Character` `Other Actor`)
  (`SceneComponent.K2_SetRelativeLocation` (`self.Plane`) (`KismetMathLibrary.MakeVector` (* 50.0 (`self.valueDirectionCharacter`)) 10.0) false false)
  (`self.SetActorEnableCollision` false)
  (set `self.scale` true))

(event `check Direction Character`
  ;[1 1 1] set value Direction Character
  (if (> (`CharacterMovementComponent.MaxWalkSpeed` (`Character.CharacterMovement` (`GameplayStatics.GetPlayerCharacter` 0))) 0.0)
    (set `self.valueDirectionCharacter` 1.0)
    (else
      (set `self.valueDirectionCharacter` -1.0))))

(fn `UserConstructionScript`)