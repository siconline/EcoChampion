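; BP_Counter is a MiniGame03 actor that detects overlapping pickups and counts those with "Metal" in their name.
; On overlap it reads the display name of the first actor of the overlapping actor's class, not necessarily the overlapping instance.
; It sets PickUpCollect by matching that name against PickUpName, and independently increments Counter when a string split finds "Metal".
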(event `self.ReceiveActorBeginOverlap`
  (params (OtherActor :type "Actor Object Reference"))
  ;[1 1 1] frägt bei overlap den actor ab der aktiviert wurde und speichert dessen namen in variablen
  (bind _outactors (`GameplayStatics.GetAllActorsOfClass` (`GameplayStatics.GetObjectClass` OtherActor)))
  (set `self.Actor Name` (`KismetSystemLibrary.GetDisplayName` (`|GetArrayItem` _outactors)))
  (set `self.PickUp Collect` (or (`.ReturnValue` (`KismetStringLibrary.Split` (`self.Actor Name`) (`self.PickUp Name`))) (`KismetStringLibrary.EqualEqual_StrStr` (`self.Actor Name`) (`self.PickUp Name`))))
  ;[1 1 1] Zählt Counter hoch
  (if (`.ReturnValue` (`KismetStringLibrary.Split` (`self.Actor Name`) "Metal"))
    (set `self.Counter` (+ (`self.Counter`) 1))))

(fn `UserConstructionScript`)