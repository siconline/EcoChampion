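; BP_ForegroundTileBottom is a bottom foreground tile for MiniGame03, displayed on a plane with collision disabled at BeginPlay.
; Three events skin the plane as a start, middle or end piece by setting its material from the matching array.
; Index selects the start and end materials directly, while the middle event picks randomly between two adjacent entries at twice Index, giving each index two variants.
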(event `self.ReceiveBeginPlay`
  (`PrimitiveComponent.SetCollisionEnabled` (`self.Plane`) "NoCollision"))

(event `Set Foreground Start Bottom`
  (`PrimitiveComponent.SetMaterial` (`self.Plane`) 0 (`|GetArrayItem` (`self.arrayMaterialStart`) (`self.index`))))

(event `Set Foreground Middle Bottom`
  (bind _index (`self.index`))
  (`PrimitiveComponent.SetMaterial` (`self.Plane`) 0 (`|GetArrayItem` (`self.arrayMaterialMiddle`) (`KismetMathLibrary.RandomIntegerInRange` (+ _index _index) (+ _index _index 1)))))

(event `Set Foreground End Bottom`
  (`PrimitiveComponent.SetMaterial` (`self.Plane`) 0 (`|GetArrayItem` (`self.arrayMaterialEnd`) (`self.index`))))

(fn `UserConstructionScript`)