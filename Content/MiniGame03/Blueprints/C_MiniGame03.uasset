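; Paper2D player character for MiniGame03 that hauls waste in a wheelbarrow to a recycling facility, with walk speed loaded from a save.
; A spawned BP_CharacterMovement receives key and mouse vertical input, while negating MaxWalkSpeed reverses horizontal travel.
; Overlaps stack indexed BP_PickUpMove actors, drop the top one on obstacles or enable facility clicks.
; Tick polls capacity, facing and boost state; carried power-ups grant HUD-tracked boost charges or extra capacity.
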(event `Set WalkSpeed`
  ;[1 1 1] Set Walk Speed character
  (`GameplayStatics.DoesSaveGameExist` "")
  (bind _returnvalue (`GameplayStatics.DoesSaveGameExist` "saveStats"))
  (if _returnvalue
    (bind _returnvalue_2 (`GameplayStatics.LoadGameFromSlot` "saveStats"))
    (set `self.svrSubClass` _returnvalue_2)
    (bind _asstat_saver (cast `/Game/Blueprints/StatSaver` (`self.svrSubClass`)))
    (bind _output_get (set `self.walkSpeed` (`/Game/Blueprints/StatSaver.speedX` _asstat_saver)))
    (set `CharacterMovementComponent.MaxWalkSpeed` _output_get (`self.CharacterMovement`))))

(event `self.ReceiveBeginPlay`
  ;[1 1 1] start Events
  (`|ExecutionSequence`
    (:`then_0`
      (if true
        (`self.SpawnActor BP_CharacterMovement`)))
    (:`then_1`
      (if true
        (`self.Set WalkSpeed`)))
    (:`then_2`
      (if true
        (`self.Set Flipbook Start`)))))

(event `Set Flipbook Start`
  ;[1 1 1] set flipbook character start
  (`PaperFlipbookComponent.SetFlipbook` (`self.Sprite`) "/Game/MiniGame03/Sprites/Character/Idle/FB_CharacterIdle8.FB_CharacterIdle8"))

(event `set flip book character`
  (bind _barrow_front (`self.barrow_front`))
  (bind _indexflipbook (`self.indexFlipbook`))
  (bind _sprite (`self.Sprite`))
  (bind _indexflipbook_2 (`self.indexFlipbook`))
  ;[1 1 1] set flip book run or idle
  ;;[1 1 1] for BP_Partner
  (if (`self.dialog`)
    _
    (elif (== (`CharacterMovementComponent.MaxWalkSpeed` (`self.CharacterMovement`)) 0.0)
      (`PaperFlipbookComponent.SetFlipbook` _sprite (`|GetArrayItem` (`self.arrayFlipbookCharacterIdle`) _indexflipbook_2))
      (`PaperSpriteComponent.SetSprite` _barrow_front (`|GetArrayItem` (`self.arraySpriteBarrowFront`) _indexflipbook_2))
      (else
        (`PaperFlipbookComponent.SetFlipbook` _sprite (`|GetArrayItem` (`self.arrayFlipbookCharacterRun`) _indexflipbook))
        (`PaperSpriteComponent.SetSprite` _barrow_front (`|GetArrayItem` (`self.arraySpriteBarrowFront`) _indexflipbook))
        ;[1 1 1] Step Sound
        (`KismetSystemLibrary.Delay` 0.4)
        (`GameplayStatics.PlaySound2D` (`|GetArrayItem` (`self.stepSounds`) (`KismetMathLibrary.RandomInteger` 4)) 8.0)))))

(event `self.ReceiveTick`
  (params (DeltaSeconds :type "Float (single-precision)"))
  ;[1 1 1] start Events
  (`|ExecutionSequence`
    (:`then_0`
      (if true
        (`self.check Sprite Rotation`)))
    (:`then_1`
      (if true
        (`self.change movement direction`)))
    (:`then_2`
      (if true
        (`self.set mouse postion`)))
    (:`then_3`
      (if true
        (`self.is mouse in range`)))
    (:`then_4`
      (if true
        (`self.set flip book character`)))
    (:`then_5`
      (if true
        (`self.check max items weelbarrow`)))
    (:`then_6`
      (if true
        (`self.checkBoost`)))
    (:`then_7`
      (if true
        (`self.Update Boost Effect Location`)))))

(event `SpawnActor BP_CharacterMovement`
  ;[1 1 1] change variable [BP_CharacterMovement] mouse input or key up/down input
  (bind _returnvalue (`|SpawnActorFromClass` "/Game/MiniGame03/Blueprints/BP_CharacterMovement.BP_CharacterMovement_C" (`KismetMathLibrary.MakeTransform` (-2000.0 0.0 0.0)) "Undefined" "OverrideRootScale" null null)))

(event `Key|Up`
  (params (Key :type "Key Structure"))
  ;[1 1 1] change variable [BP_CharacterMovement] mouse input or key up/down input
  (:`Pressed`
    (`/Game/MiniGame03/Blueprints/BP_CharacterMovement.keyUp` (stale `SpawnActor BP_CharacterMovement` _returnvalue))))

(event `is mouse in range`
  (bind _z (.z (`self.currentMousePosition`)))
  (bind _z_2 (.z (`self.K2_GetActorLocation`)))
  ;[1 1 1] check mouse position for is mouse in range --> Input Action Mouse Button
  (if (or (> _z (+ _z_2 100.0)) (< _z (+ _z_2 -100.0)))
    (set `self.checkMousePosition` true)
    (else
      (set `self.checkMousePosition` false))))

(event `InputAction|MouseButton`
  (params (Key :type "Key Structure"))
  ;[1 1 1] change variable [BP_CharacterMovement] mouse input or key up/down input
  (:`Pressed`
    (`/Engine/EditorBlueprintResources/StandardMacros.IsValid` (stale `SpawnActor BP_CharacterMovement` _returnvalue)
      (:`Is Valid`
        (if (`self.checkMousePosition`) :!label _label
          (`/Game/MiniGame03/Blueprints/BP_CharacterMovement.enableMoveZ` (stale `SpawnActor BP_CharacterMovement` _returnvalue))))))
  (:`Released`
    (`/Engine/EditorBlueprintResources/StandardMacros.IsValid` (stale `SpawnActor BP_CharacterMovement` _returnvalue)
      (:`Is Valid`
        (goto _label)))))

(event `Key|Down`
  (params (Key :type "Key Structure"))
  ;[1 1 1] change variable [BP_CharacterMovement] mouse input or key up/down input
  (:`Pressed`
    (`/Game/MiniGame03/Blueprints/BP_CharacterMovement.keyDown` (stale `SpawnActor BP_CharacterMovement` _returnvalue))))

(event `Spawn BP_PickUpMove`
  (params (`Other Actor` :type "Actor Object Reference"))
  (bind _actorpickupmove (`self.actorPickUpMove`))
  ;[1 1 1] spawn pickup move [BP_PickUpMove]
  (bind _asbp_pick_up (cast `/Game/MiniGame03/Blueprints/BP_PickUp` `Other Actor`))
  (bind _returnvalue (`KismetArrayLibrary.Array_Add` (`self.arrayPickUps`) _actorpickupmove))
  (bind _returnvalue_2 (`|SpawnActorFromClass` _actorpickupmove (`KismetMathLibrary.MakeTransform` (0.0 0.0 0.0)) "Undefined" "OverrideRootScale" null null))
  ;;[1 1 1] set material on PickUpMove
  (bind _asbp_pick_up_move (cast `/Game/MiniGame03/Blueprints/BP_PickUpMove` _returnvalue_2))
  (set `/Game/MiniGame03/Blueprints/BP_PickUpMove.indexPickUpMove` _returnvalue _asbp_pick_up_move) ; set z position
  (set `/Game/MiniGame03/Blueprints/BP_PickUpMove.index` (`/Game/MiniGame03/Blueprints/BP_PickUp.index` _asbp_pick_up) _asbp_pick_up_move))

(event `self.ReceiveActorBeginOverlap`
  (params (OtherActor :type "Actor Object Reference"))
  ;[1 1 1] start Events
  (`|ExecutionSequence`
    (:`then_0`
      (if true
        (`self.EnableDisableClickOnBP_RecyclingFacility` OtherActor)))
    (:`then_1`
      (if true
        (`self.Spawn BP_PickUpMove` OtherActor)))
    (:`then_2`
      (if true
        (`self.To lose PickUpMove` OtherActor)))))

(event `remove recycled waste`
  (params (`Other Actor` :type "Actor Object Reference"))
  (bind _arraypickups (`self.arrayPickUps`))
  ;[1 1 1] remove recycled waste  --> referenz BP_RecyclingFacility --> start animation
  (bind _outactors (`GameplayStatics.GetAllActorsOfClass` "/Game/MiniGame03/Blueprints/BP_PickUpMove.BP_PickUpMove_C"))
  (bind (_arrayindex _arrayelement) (`/Engine/EditorBlueprintResources/StandardMacros.ReverseForEachLoop` _outactors)
    (:`LoopBody`
      (bind _indexpickupmove (`/Game/MiniGame03/Blueprints/BP_PickUpMove.indexPickUpMove` _arrayelement))
      (if (> _indexpickupmove (`self.saveIndex`))
        (set `self.saveIndex` _indexpickupmove)))
    (:`Completed`
      (bind _outactors_2 (`GameplayStatics.GetAllActorsOfClass` "/Game/MiniGame03/Blueprints/BP_PickUpMove.BP_PickUpMove_C"))
      (bind (_arrayindex_2 _arrayelement_2) (`/Engine/EditorBlueprintResources/StandardMacros.ReverseForEachLoop` _outactors_2)
        (:`LoopBody`
          (if (== (`/Game/MiniGame03/Blueprints/BP_PickUpMove.indexPickUpMove` _arrayelement_2) (`self.saveIndex`))
            (`/Engine/EditorBlueprintResources/StandardMacros.IsValid` _arrayelement_2
              (:`Is Valid`
                (`/Engine/EditorBlueprintResources/StandardMacros.Do N` 1 :!label _label_2
                  (:`Exit`
                    (`KismetArrayLibrary.Array_Remove` _arraypickups (`KismetArrayLibrary.Array_LastIndex` _arraypickups))
                    (if (not (== (`self.saveIndex`) -1))
                      (set `self.saveIndex` (+ (`self.saveIndex`) -1))
                      (bind _asbp_recycling_facility (cast `/Game/MiniGame03/Blueprints/BP_RecyclingFacility` `Other Actor`))
                      (set `/Game/MiniGame03/Blueprints/BP_RecyclingFacility.materialWasteIndex` (`/Game/MiniGame03/Blueprints/BP_PickUpMove.index` _arrayelement_2) _asbp_recycling_facility)
                      (`/Game/MiniGame03/Blueprints/BP_PickUpMove.destroy actor` _arrayelement_2)
                      (`KismetSystemLibrary.Delay` 0.2)
                      (goto _label_2 :!via `Reset`))))))))))))

(event `Key|Right`
  (params (Key :type "Key Structure"))
  ;[1 1 1] start Events
  (:`Pressed`
    (`|ExecutionSequence`
      (:`then_0`
        (if true
          (`self.reverse direction by player`)))))
  (:`Released`
    (`|ExecutionSequence`
      (:`then_0`
        (if true
          (`self.Reset reverse direction by player`))))))

(event `To lose PickUpMove`
  (params (`Other Actor` :type "Actor Object Reference"))
  (bind _arraypickups (`self.arrayPickUps`))
  ;[1 1 1] to lose PickUpMove if collision with obstacle
  (bind _asbp_obstacle (cast `/Game/MiniGame03/Blueprints/BP_Obstacle` `Other Actor`))
  (bind _index (`/Game/MiniGame03/Blueprints/BP_Obstacle.index` _asbp_obstacle))
  (if (or (== _index 0) (== _index 1))
    (bind _outactors (`GameplayStatics.GetAllActorsOfClass` "/Game/MiniGame03/Blueprints/BP_PickUpMove.BP_PickUpMove_C"))
    (for _array_element _outactors
      (bind _indexpickupmove (`/Game/MiniGame03/Blueprints/BP_PickUpMove.indexPickUpMove` _array_element))
      (if (> _indexpickupmove (`self.saveIndex`))
        (set `self.saveIndex` _indexpickupmove)))
    (bind _outactors_2 (`GameplayStatics.GetAllActorsOfClass` "/Game/MiniGame03/Blueprints/BP_PickUpMove.BP_PickUpMove_C"))
    (for _array_element_2 _outactors_2
      (if (== (`/Game/MiniGame03/Blueprints/BP_PickUpMove.indexPickUpMove` _array_element_2) (`self.saveIndex`))
        (`/Engine/EditorBlueprintResources/StandardMacros.IsValid` _array_element_2
          (:`Is Valid`
            (`/Engine/EditorBlueprintResources/StandardMacros.Do N` 1 :!label _label_3
              (:`Exit`
                (`/Game/MiniGame03/Blueprints/BP_PickUpMove.Animation To lose PickUpMove` _array_element_2)
                (`KismetArrayLibrary.Array_Remove` _arraypickups (`KismetArrayLibrary.Array_LastIndex` _arraypickups))
                (if (not (== (`self.saveIndex`) -1))
                  (set `self.saveIndex` (+ (`self.saveIndex`) -1))
                  (`KismetSystemLibrary.Delay` 0.2)
                  (goto _label_3 :!via `Reset`))))))))))

(event `EnableDisableClickOnBP_RecyclingFacility`
  (params (`Other Actor` :type "Actor Object Reference"))
  ;[1 1 1] enable to click the Recycling Facility
  (bind _asbp_recycling_facility (cast `/Game/MiniGame03/Blueprints/BP_RecyclingFacility` `Other Actor`))
  ;;[1 1 1] disable to click on Recycling Facility when PickUpMove is empty
  (bind _outactors (`GameplayStatics.GetAllActorsOfClass` "/Game/MiniGame03/Blueprints/BP_PickUpMove.BP_PickUpMove_C"))
  (for (_ _array_index) _outactors
    (if (>= _array_index 0)
      (set `/Game/MiniGame03/Blueprints/BP_RecyclingFacility.clickable` true _asbp_recycling_facility))))

(event `show Sp_Ecoboost`
  ;[1 1 1] show and hide SP_Powerups / Sp_ecoboost -- Sp_toolbox
  (`SceneComponent.SetVisibility` (`self.Sp_ecoboost`) true false))

(event `show Sp_Toolbox`
  ;[1 1 1] show and hide SP_Powerups / Sp_ecoboost -- Sp_toolbox
  (`SceneComponent.SetVisibility` (`self.Sp_toolbox`) true false))

(event `check Sprite Rotation`
  (bind _sp_ecoboost (`self.Sp_ecoboost`))
  (bind _sp_toolbox (`self.Sp_toolbox`))
  (bind _maxwalkspeed (`CharacterMovementComponent.MaxWalkSpeed` (`self.CharacterMovement`)))
  ;[1 1 1] check sprite rotation
  (if (< _maxwalkspeed 0.0)
    (`SceneComponent.K2_SetRelativeRotation` (`self.Sprite`) (`KismetMathLibrary.MakeRotator` 0.0 0.0 180.0) false false)
    (`SceneComponent.K2_SetRelativeRotation` (`self.barrow_front`) (`KismetMathLibrary.MakeRotator` 0.0 0.0 180.0) false false)
    (`SceneComponent.K2_SetRelativeRotation` (`self.barrow_front_update`) (`KismetMathLibrary.MakeRotator` 0.0 0.0 180.0) false false)
    ;;[1 1 1] powerups
    (`SceneComponent.K2_SetRelativeTransform` _sp_ecoboost (`KismetMathLibrary.MakeTransform` (-103.846481 8.0 -5.67571) (struct :`Yaw` 180.0)) false false)
    (`SceneComponent.K2_SetRelativeTransform` _sp_toolbox (`KismetMathLibrary.MakeTransform` (-96.292969 5.0 4.134978) (struct :`Yaw` 180.0)) false false)
    (elif (> _maxwalkspeed 0.0)
      (`SceneComponent.K2_SetRelativeRotation` (`self.Sprite`) (`KismetMathLibrary.MakeRotator` 0.0) false false)
      (`SceneComponent.K2_SetRelativeRotation` (`self.barrow_front`) (`KismetMathLibrary.MakeRotator` 0.0) false false)
      (`SceneComponent.K2_SetRelativeRotation` (`self.barrow_front_update`) (`KismetMathLibrary.MakeRotator` 0.0) false false)
      (`SceneComponent.K2_SetRelativeTransform` _sp_ecoboost (`KismetMathLibrary.MakeTransform` (103.846481 8.0 -5.67571)) false false)
      (`SceneComponent.K2_SetRelativeTransform` _sp_toolbox (`KismetMathLibrary.MakeTransform` (96.292969 5.0 4.134978)) false false))))

(event `hide Sp_Ecoboost`
  ;[1 1 1] show and hide SP_Powerups / Sp_ecoboost -- Sp_toolbox
  (`SceneComponent.SetVisibility` (`self.Sp_ecoboost`) false false))

(event `hide Sp_Toolbox`
  ;[1 1 1] show and hide SP_Powerups / Sp_ecoboost -- Sp_toolbox
  (`SceneComponent.SetVisibility` (`self.Sp_toolbox`) false false))

(event `change movement direction`
  (bind _charactermovement (`self.CharacterMovement`))
  ;[1 1 1] change movement direction by X -300
  (if (<= (.x (`self.K2_GetActorLocation`)) -300.0)
    (`|ExecutionSequence`
      (:`then_0`
        (`/Engine/EditorBlueprintResources/StandardMacros.Do N` 1 :!label _label_4
          (:`Exit`
            (bind _output_get (set `self.saveMaxWalkSpeed` (`CharacterMovementComponent.MaxWalkSpeed` _charactermovement))))))
      (:`then_1`
        (set `CharacterMovementComponent.MaxWalkSpeed` 0.0 _charactermovement)
        (`KismetSystemLibrary.Delay` 2.0)
        (set `CharacterMovementComponent.MaxWalkSpeed` (* _output_get -1.0) _charactermovement)))
    (else
      (goto _label_4 :!via `Reset`))))

(event `set mouse postion`
  ;[1 1 1] set current mouse position
  (set `self.currentMousePosition` (`KismetMathLibrary.MakeVector` (.x (`.Location` (`GameplayStatics.BreakHitResult` (`PlayerController.GetHitResultUnderCursorByChannel` (`GameplayStatics.GetPlayerController` 0) "TraceTypeQuery1" true)))) (.y (`.Location` (`GameplayStatics.BreakHitResult` (`PlayerController.GetHitResultUnderCursorByChannel` (`GameplayStatics.GetPlayerController` 0) "TraceTypeQuery1" true)))) (.z (`.Location` (`GameplayStatics.BreakHitResult` (`PlayerController.GetHitResultUnderCursorByChannel` (`GameplayStatics.GetPlayerController` 0) "TraceTypeQuery1" true)))))))

(event `check max items weelbarrow`
  ;[1 1 1] check max items at weelbarrow and manipulate PickUps on playfeld
  (bind _outactors (`GameplayStatics.GetAllActorsOfClass` "/Game/MiniGame03/Blueprints/BP_PickUpMove.BP_PickUpMove_C"))
  (set `self.counterWeelbarrow` (`KismetArrayLibrary.Array_LastIndex` _outactors))
  (if (>= (`self.counterWeelbarrow`) (- (`self.maxItemsCharacter`) 1))
    (bind _outactors_2 (`GameplayStatics.GetAllActorsOfClass` "/Game/MiniGame03/Blueprints/BP_PickUp.BP_PickUp_C"))
    (for _array_element _outactors_2
      (`/Engine/EditorBlueprintResources/StandardMacros.IsValid` _array_element
        (:`Is Valid`
          (`/Game/MiniGame03/Blueprints/BP_PickUp.full weelbarrow` _array_element))))
    (else
      (bind _outactors_3 (`GameplayStatics.GetAllActorsOfClass` "/Game/MiniGame03/Blueprints/BP_PickUp.BP_PickUp_C"))
      (for _array_element_2 _outactors_3
        (`/Engine/EditorBlueprintResources/StandardMacros.IsValid` _array_element_2
          (:`Is Valid`
            (`/Game/MiniGame03/Blueprints/BP_PickUp.empty weelbarrow` _array_element_2)))))))

(event `PowerUpWheelbarrow`
  ;[1 1 1] PowerUpWheelbarrow
  (set `self.maxItemsCharacter` (+ (`self.maxItemsCharacter`) 1)))

(event `carryBoost`
  ;[1 1 1] Set Upgrade States
  (set `self.carriesBoost` true)
  (`self.show Sp_Ecoboost`))

(event `checkBoost`
  ;[1 1 1] set visibility barrow upgrate and hud boost button by boost Charges
  (if (`self.hasBoost`)
    (if (== (`self.boostCharges`) 0)
      (`/Engine/EditorBlueprintResources/StandardMacros.Do N` 1 :!label _label_5
        (:`Exit`
          (bind (_direction _visibility) (`Timeline|animation Visibilty` :!via `PlayFromStart`)
            (:`Update`
              (if (< _visibility 0.0)
                (`SceneComponent.SetVisibility` (`self.barrow_front_update`) false false)
                (goto _label_6 :!via `HASN'T BOOST`)
                (else
                  (`SceneComponent.SetVisibility` (`self.barrow_front_update`) true false)
                  (`self.castToHUD_MiniGame03` :!label _label_6)))))))
      (else
        (`SceneComponent.SetVisibility` (`self.barrow_front_update`) true false)
        (`self.castToHUD_MiniGame03` :!label _label_7
          (:`OUT`
            (`self.reset Animation Visibility`)))))
    (else
      (`SceneComponent.SetVisibility` (`self.barrow_front_update`) false false)
      (goto _label_7 :!via `HASN'T BOOST`))))

(event `reset Animation Visibility`
  ;[1 1 1] set visibility barrow upgrate and hud boost button by boost Charges
  (goto _label_5 :!via `Reset`))

(event `carryWheelbarrowUpgrade`
  ;[1 1 1] Set Upgrade States
  (set `self.carriesWheelbarrowUpgrade` true)
  (`self.show Sp_Toolbox`))

(event `removeCarryBoost`
  ;[1 1 1] Set Upgrade States
  (if (`self.carriesBoost`)
    (set `self.carriesBoost` false)
    (if (`self.hasBoost`)
      (set `self.boostCharges` 3)
      (`self.castToHUD_MiniGame03` :!via `BOOST THREE` :!label _label_8
        (:`OUT`
          _))
      (else
        (set `self.hasBoost` true)
        (set `self.boostCharges` 3)
        (goto _label_8 :!via `BOOST THREE`)))
    (`self.Respawn Boost`)
    (`self.hide Sp_Ecoboost`)
    ;;[1 1 1] play NPC win animation
    (`self.castToPartner` :!label _label_9
      (:`OUT`
        (`KismetSystemLibrary.Delay` 2.0)
        (`self.castToPartner` :!via `SET FLIPBOOK IDLE`)))))

(event `removeCarryWheelbarrowUpgrade`
  ;[1 1 1] Set Upgrade States
  (if (`self.carriesWheelbarrowUpgrade`)
    (set `self.carriesWheelbarrowUpgrade` false)
    (`self.PowerUpWheelbarrow`)
    (`GameplayStatics.GetAllActorsOfClass` null)
    (`self.Respawn Upgrade`)
    (`self.hide Sp_Toolbox`)
    (set `self.indexFlipbook` 1)
    (goto _label_9)))

(event `Respawn Boost`
  ;[1 1 1] Respawn PowerUps
  (bind _returnvalue (`|SpawnActorFromClass` "/Game/MiniGame03/Blueprints/BP_PowerUp.BP_PowerUp_C" (`KismetMathLibrary.MakeTransform` (`KismetMathLibrary.MakeVector` (`KismetMathLibrary.Conv_IntToDouble` (`KismetMathLibrary.RandomIntegerInRange` 1500 (- (* (`self.backgroundWidthC`) (`self.levelLengthC`)) 1500))) 200.0 (`|GetArrayItem` (`self.arrayPickUpsPositionZC`) (`KismetMathLibrary.RandomIntegerInRange` 0 4)))) "Undefined" "OverrideRootScale" null null))
  (bind _asbp_power_up (cast `/Game/MiniGame03/Blueprints/BP_PowerUp` _returnvalue))
  (`/Game/MiniGame03/Blueprints/BP_PowerUp.Set Type Boost` _asbp_power_up))

(event `Respawn Upgrade`
  ;[1 1 1] Respawn PowerUps
  (bind _returnvalue (`|SpawnActorFromClass` "/Game/MiniGame03/Blueprints/BP_PowerUp.BP_PowerUp_C" (`KismetMathLibrary.MakeTransform` (`KismetMathLibrary.MakeVector` (`KismetMathLibrary.Conv_IntToDouble` (`KismetMathLibrary.RandomIntegerInRange` 1500 (- (* (`self.backgroundWidthC`) (`self.levelLengthC`)) 1500))) 200.0 (`|GetArrayItem` (`self.arrayPickUpsPositionZC`) (`KismetMathLibrary.RandomIntegerInRange` 0 4)))) "Undefined" "OverrideRootScale" null null))
  (bind _asbp_power_up (cast `/Game/MiniGame03/Blueprints/BP_PowerUp` _returnvalue))
  (`/Game/MiniGame03/Blueprints/BP_PowerUp.Set Type Upgrade` _asbp_power_up))

(event `Key|RightShift`
  (params (Key :type "Key Structure"))
  ;[1 1 1] Boost Activation
  (:`Pressed`
    (if (`self.hasBoost`) :!label _label_10
      (if (> (`self.boostCharges`) 0)
        (`self.Show Boost Effect`)
        (`self.castToChracterMovement`
          (:`OUT`
            (bind _output_get (set `self.boostCharges` (- (`self.boostCharges`) 1)))
            (switch `int` _output_get
              (:`0`
                (`self.castToHUD_MiniGame03` :!via `BOOST ZERO` :!label _label_11))
              (:`1`
                (goto _label_11 :!via `BOOST ONE`))
              (:`2`
                (goto _label_11 :!via `BOOST TWO`)))))))))

(event `Boost`
  ;[1 1 1] Boost Activation
  (goto _label_10))

(event `reverse direction by player`
  (bind _charactermovement (`self.CharacterMovement`))
  (bind _maxwalkspeed (`CharacterMovementComponent.MaxWalkSpeed` _charactermovement))
  ;[1 1 1] reverse direction by player input
  (if (and (< _maxwalkspeed 0.0) (< (.x (`self.K2_GetActorLocation`)) (`KismetMathLibrary.Conv_IntToDouble` (+ (* (`self.backgroundWidthC`) (`self.levelLengthC`)) 1))))
    (`/Engine/EditorBlueprintResources/StandardMacros.Do N` 1 :!label _label_12
      (:`Exit`
        (set `CharacterMovementComponent.MaxWalkSpeed` (* _maxwalkspeed -1.0) _charactermovement)))))

(event `Reset reverse direction by player`
  ;[1 1 1] reverse direction by player input
  (`KismetSystemLibrary.Delay` 1.0)
  (goto _label_12 :!via `Reset`))

(event `Update Boost Effect Location`
  ;[1 1 1] show boost effect
  (if (`self.updateBoostEffectLocation`)
    (`SceneComponent.K2_SetRelativeLocation` (stale `Show Boost Effect` _returnvalue) (`KismetMathLibrary.MakeVector` (.x (`self.K2_GetActorLocation`)) (+ (.y (`self.K2_GetActorLocation`)) 100.0) (+ (.z (`self.K2_GetActorLocation`)) -30.0)) false false)))

(event `Show Boost Effect`
  ;[1 1 1] show boost effect
  (bind _returnvalue (`GameplayStatics.SpawnEmitterAtLocation` "/Game/Particles/P_Boost.P_Boost"))
  (set `self.updateBoostEffectLocation` true)
  (`KismetSystemLibrary.Delay` 1.0)
  (set `self.updateBoostEffectLocation` false)
  (`ActorComponent.K2_DestroyComponent` _returnvalue))

(fn `UserConstructionScript`)