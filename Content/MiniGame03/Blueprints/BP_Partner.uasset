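; BP_Partner is a MiniGame03 actor that strips carry upgrades from C_MiniGame03 when it enters the partner's Box volume.
; On begin overlap, it checks that the other actor is the first C_MiniGame03 overlapping the Box.
; It then looks up the first C_MiniGame03 in the level, rather than using the overlapping reference, and calls RemoveCarryBoost and RemoveCarryWheelbarrowUpgrade on it.
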(event `self.ReceiveActorBeginOverlap`
  (params (OtherActor :type "Actor Object Reference"))
  (if (== (`|GetArrayItem` (`PrimitiveComponent.GetOverlappingActors` (`self.Box`) "/Game/MiniGame03/Blueprints/C_MiniGame03.C_MiniGame03_C")) OtherActor)
    (`|ExecutionSequence`
      (:`then_0`
        (bind _outactors (`GameplayStatics.GetAllActorsOfClass` "/Game/MiniGame03/Blueprints/C_MiniGame03.C_MiniGame03_C"))
        (bind _asc_mini_game_03 (cast `/Game/MiniGame03/Blueprints/C_MiniGame03` (`|GetArrayItem` _outactors)))
        (`/Game/MiniGame03/Blueprints/C_MiniGame03.removeCarryBoost` _asc_mini_game_03))
      (:`then_1`
        (bind _outactors_2 (`GameplayStatics.GetAllActorsOfClass` "/Game/MiniGame03/Blueprints/C_MiniGame03.C_MiniGame03_C"))
        (bind _asc_mini_game_03_2 (cast `/Game/MiniGame03/Blueprints/C_MiniGame03` (`|GetArrayItem` _outactors_2)))
        (`/Game/MiniGame03/Blueprints/C_MiniGame03.removeCarryWheelbarrowUpgrade` _asc_mini_game_03_2)))))

(fn `UserConstructionScript`)