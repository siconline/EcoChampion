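; MiniGame03 obstacle whose Index selects its collision effect, sound, material and scale.
; Indices 0–1 freeze the character, disable collision and input, then Tick pushes and blinks the player until a set distance restores control.
; Indices 2–3 quarter walk speed and block input until overlap ends.
; The saved localisation picks the material set on BeginPlay, and a Tick check destroys the obstacle when it overlaps a BP_PowerUp.
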(event `playSoundOnCollision`
  (params (`Other Actor` :type "Actor Object Reference"))
  ;[1 1 1] SOUNDS
  (cast `/Game/MiniGame03/Blueprints/C_MiniGame03` `Other Actor`)
  (`GameplayStatics.PlaySound2D` (`|GetArrayItem` (`self.arraySound`) (`self.index`))))

(event `self.ReceiveBeginPlay`
  ;[1 1 1] start Events
  (`|ExecutionSequence`
    (:`then_0`
      (if true
        (`self.SetMaterialByLocalisation`)))))

(event `Save MaxWalkSpeed`
  (params (`Other Actor` :type "Actor Object Reference"))
  ;[1 1 1] save MaxWalkSpeed
  (bind _ascharacter (cast `Character` `Other Actor`))
  (`/Engine/EditorBlueprintResources/StandardMacros.Do N` 1 :!label _label
    (:`Exit`
      (set `self.saveMaxWalkSpeed` (`CharacterMovementComponent.MaxWalkSpeed` (`Character.CharacterMovement` _ascharacter))))))

(event `reset`
  ;[1 1 1] save MaxWalkSpeed
  (goto _label :!via `Reset`))

(event `self.ReceiveTick`
  (params (DeltaSeconds :type "Float (single-precision)"))
  ;[1 1 1] start Events
  (`|ExecutionSequence`
    (:`then_0`
      (if true
        (`self.Play Animation Damage`)))
    (:`then_1`
      (if true
        (`self.check walk direction set throwback`)))
    (:`then_2`
      (if true
        (`self.destroy overlapping actor`)))))

(event `Set Material Obstacle`
  ;[1 1 1] set standard material
  (`PrimitiveComponent.SetMaterial` (`self.StaticMesh`) 0 (`|GetArrayItem` (`self.arrayMaterial`) (`self.index`))))

(event `SetMaterialByLocalisation`
  ;[1 1 1] set Material by localisation
  (bind _returnvalue (`GameplayStatics.LoadGameFromSlot` "saveStats"))
  (bind _asstat_saver (cast `/Game/Blueprints/StatSaver` _returnvalue))
  (bind _local (`/Game/Blueprints/StatSaver.local` _asstat_saver))
  (set `self.indexLocalisation` _local)
  (if (== _local 1)
    (set `self.arrayMaterial` (`self.arrayMaterial_a`))
    (else
      (set `self.arrayMaterial` (`self.arrayMaterial_m_d`)))))

(event `Play Animation Damage`
  (bind _returnvalue (`GameplayStatics.GetPlayerCharacter` 0))
  (bind _x (.x (`self.K2_GetActorLocation` _returnvalue)))
  ;[1 1 1] animation damage
  (if (`self.damage`)
    (`self.K2_SetActorRelativeLocation` _returnvalue (`KismetMathLibrary.MakeVector` (+ _x (`self.throwbackValue`)) (.y (`self.K2_GetActorLocation` _returnvalue)) (.z (`self.K2_GetActorLocation` _returnvalue))) false false)
    (`KismetSystemLibrary.Delay` 0.1)
    (bind _isa (`/Engine/EditorBlueprintResources/StandardMacros.FlipFlop`)
      (:`A`
        _)
      (:`B`
        _))
    (`self.SetActorHiddenInGame` (`GameplayStatics.GetPlayerCharacter` 0) _isa)
    (bind _returnvalue_2 (- _x (.x (stale `EnableDamage` _output_get))))
    (if (or (<= _returnvalue_2 -300.0) (>= _returnvalue_2 300.0))
      (`self.DisableDamage`))))

(event `self.ReceiveActorBeginOverlap`
  (params (OtherActor :type "Actor Object Reference"))
  ;[1 1 1] start Events
  (`|ExecutionSequence`
    (:`then_0`
      (if true
        (`self.Save MaxWalkSpeed` OtherActor)))
    (:`then_1`
      (if true
        (`self.Start Event -enableDamage-` OtherActor)))
    (:`then_2`
      (if true
        (`self.Start Event -enableMotion` OtherActor)))
    (:`then_3`
      (if true
        (`self.playSoundOnCollision` OtherActor)))))

(event `EnableDamage`
  ;[1 1 1] animation damage
  (set `self.damage` true)
  (bind _output_get (set `self.saveCurrentPosition` (`self.K2_GetActorLocation` (`GameplayStatics.GetPlayerCharacter` 0)))))

(event `DisableDamage`
  (bind _returnvalue (`GameplayStatics.GetPlayerCharacter` 0))
  ;[1 1 1] reset animation damage
  (set `self.damage` false)
  (`self.SetActorHiddenInGame` _returnvalue false)
  (`KismetSystemLibrary.Delay` 0.5)
  (set `CharacterMovementComponent.MaxWalkSpeed` (`self.saveMaxWalkSpeed`) (`Character.CharacterMovement` _returnvalue))
  (`self.EnableInput` _returnvalue (`GameplayStatics.GetPlayerController` 0))
  (`self.reset`)
  (bind _ascharacter (cast `Character` (`GameplayStatics.GetPlayerCharacter` 0)))
  (`self.SetActorEnableCollision` _ascharacter true))

(event `Start Event -enableDamage-`
  (params (`Other Actor` :type "Actor Object Reference"))
  (bind _index (`self.index`))
  ;[1 1 1] start event enableDamage by index 0
  (if (or (== _index 0) (== _index 1))
    (bind _ascharacter (cast `Character` `Other Actor`))
    (`self.SetActorEnableCollision` _ascharacter false)
    (set `CharacterMovementComponent.MaxWalkSpeed` 0.0 (`Character.CharacterMovement` _ascharacter))
    (`self.DisableInput` _ascharacter (`GameplayStatics.GetPlayerController` 0))
    (`self.EnableDamage`)))

(event `Start Event -enableMotion`
  (params (`Other Actor` :type "Actor Object Reference"))
  (bind _index (`self.index`))
  ;[1 1 1] start event enableMotion by index 2 or 3
  (if (or (== _index 2) (== _index 3))
    (bind _ascharacter (cast `Character` `Other Actor`))
    (bind _charactermovement (`Character.CharacterMovement` _ascharacter))
    (set `CharacterMovementComponent.MaxWalkSpeed` (* (`CharacterMovementComponent.MaxWalkSpeed` _charactermovement) 0.25) _charactermovement)
    (`self.DisableInput` _ascharacter (`GameplayStatics.GetPlayerController` 0))))

(event `self.ReceiveActorEndOverlap`
  (params (OtherActor :type "Actor Object Reference"))
  (bind _index (`self.index`))
  ;[1 1 1] start event enableMotion by index 2 or 3
  (if (or (== _index 2) (== _index 3))
    (bind _ascharacter (cast `Character` OtherActor))
    (bind _charactermovement (`Character.CharacterMovement` _ascharacter))
    (set `CharacterMovementComponent.MaxWalkSpeed` (* (`CharacterMovementComponent.MaxWalkSpeed` _charactermovement) 4.0) _charactermovement)
    (`self.EnableInput` (`GameplayStatics.GetPlayerCharacter` 0) (`GameplayStatics.GetPlayerController` 0))
    (`KismetSystemLibrary.Delay` 1.0)
    (`self.reset`)))

(event `check walk direction set throwback`
  (bind _maxwalkspeed (`CharacterMovementComponent.MaxWalkSpeed` (`Character.CharacterMovement` (`GameplayStatics.GetPlayerCharacter` 0))))
  ;[1 1 1] check walk direction and set throwback value
  (if (> _maxwalkspeed 0.0)
    (set `self.throwbackValue` -4.0)
    (elif (< _maxwalkspeed 0.0)
      (set `self.throwbackValue` 4.0))))

(event `Set Actor Scale`
  (bind _index (`self.index`))
  (bind _x (.x (`self.K2_GetActorLocation`)))
  (bind _y (.y (`self.K2_GetActorLocation`)))
  (bind _returnvalue (+ (.z (`self.K2_GetActorLocation`)) -40.0))
  ;[1 1 1] set Actor Scale by Index
  (if (or (== _index 0) (== _index 1))
    (if (== (`self.indexLocalisation`) 1)
      (if (== (`self.index`) 0)
        (`self.K2_SetActorTransform` (`KismetMathLibrary.MakeTransform` (`self.K2_GetActorLocation`) (struct) (2.5 2.0 1.0)))
        (`SceneComponent.SetRelativeScale3D` (`self.Box`) (0.6 1.0 1.0))
        (else
          (`self.K2_SetActorTransform` (`KismetMathLibrary.MakeTransform` (`self.K2_GetActorLocation`) (struct) (3.73 2.0 1.0)))
          (`SceneComponent.SetRelativeScale3D` (`self.Box`) (1.0 1.0 1.0))))
      (else
        (`self.K2_SetActorTransform` (`KismetMathLibrary.MakeTransform` (`self.K2_GetActorLocation`) (struct) (0.81 2.3 3.0)))
        (`SceneComponent.SetRelativeScale3D` (`self.Box`) (0.5 1.0 1.0))))
    (elif (== (`self.index`) 2)
      (`self.K2_SetActorTransform` (`KismetMathLibrary.MakeTransform` (`KismetMathLibrary.MakeVector` _x _y _returnvalue) (struct) (1.86 1.2 1.0)))
      (`SceneComponent.SetRelativeScale3D` (`self.Box`) (0.8 0.8 0.8))
      (else
        (`self.K2_SetActorTransform` (`KismetMathLibrary.MakeTransform` (`KismetMathLibrary.MakeVector` _x _y _returnvalue) (struct) (1.92 0.96 1.0)))
        (`SceneComponent.SetRelativeScale3D` (`self.Box`) (0.8 0.8 0.8))))))

(event `destroy overlapping actor`
  (bind _overlappingactors (`PrimitiveComponent.GetOverlappingActors` (`self.Box`) "/Game/MiniGame03/Blueprints/BP_PowerUp.BP_PowerUp_C"))
  ;[1 1 1] destroy overlapping actor
  (if (`KismetArrayLibrary.Array_Contains` _overlappingactors (`|GetArrayItem` _overlappingactors (`KismetArrayLibrary.Array_LastIndex` _overlappingactors)))
    (`self.K2_DestroyActor`)))

(fn `UserConstructionScript`)