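; BP_Flowers is a MiniGame03 flower actor whose Plane switches from a dirty material to a clean one once no pickups cover it.
; BeginPlay applies M_FlowerDirty to the Plane.
; Every Tick queries the Box for overlapping BP_PickUp actors and sets M_Flower when the array lacks its own last element, effectively an empty-array check.
; Nothing restores the dirty material afterward.
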(event `self.ReceiveBeginPlay`
  (`PrimitiveComponent.SetMaterial` (`self.Plane`) 0 "/Game/Materials/M_FlowerDirty.M_FlowerDirty"))

(event `self.ReceiveTick`
  (params (DeltaSeconds :type "Float (single-precision)"))
  (bind _overlappingactors (`PrimitiveComponent.GetOverlappingActors` (`self.Box`) "/Game/MiniGame03/Blueprints/BP_PickUp.BP_PickUp_C"))
  (if (not (`KismetArrayLibrary.Array_Contains` _overlappingactors (`|GetArrayItem` _overlappingactors (`KismetArrayLibrary.Array_LastIndex` _overlappingactors))))
    (`PrimitiveComponent.SetMaterial` (`self.Plane`) 0 "/Game/Materials/M_Flower.M_Flower")))

(fn `UserConstructionScript`)