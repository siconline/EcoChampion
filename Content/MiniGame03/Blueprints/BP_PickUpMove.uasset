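; BP_PickUpMove is a MiniGame03 actor that shows a pickup following the first player character, apparently as part of a carried stack.
; Every Tick it snaps to the player's location plus fixed world-axis offsets, with height and a slight Y shift growing with IndexPickUpMove.
; The same Tick reapplies the mesh material, chosen from ArrayMaterial by a separate Index variable.
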(event `self.ReceiveTick`
  (params (DeltaSeconds :type "Float (single-precision)"))
  (set `self.offsetZ` (* (`self.indexPickUpMove`) 40.0))
  (set `self.offsetY` (`KismetMathLibrary.Conv_IntToDouble` (+ (`self.indexPickUpMove`) 1)))
  (`PrimitiveComponent.SetMaterial` (`self.StaticMesh`) 0 (`|GetArrayItem` (`self.arrayMaterial`) (`self.index`)))
  (`self.K2_SetActorLocation` (`KismetMathLibrary.MakeVector` (+ (.x (`self.K2_GetActorLocation` (`GameplayStatics.GetPlayerCharacter` 0))) 40.0) (+ (.y (`self.K2_GetActorLocation` (`GameplayStatics.GetPlayerCharacter` 0))) (`self.offsetY`) 5.0) (+ (.z (`self.K2_GetActorLocation` (`GameplayStatics.GetPlayerCharacter` 0))) (`self.offsetZ`) 25.0))))

(fn `UserConstructionScript`)