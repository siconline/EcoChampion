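; BP_CharacterMovement drives the player character in MiniGame03, moving it along X every tick at MaxWalkSpeed unless Dialog is set.
; Key up/down events hop it between five height lanes with a slight Y shift, and SetBoost plays a sound and multiplies speed for one second.
; MaxStepHeight is repurposed as a per-tick Z step for mouse-steered vertical movement, whose Tick branches are switched off.
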(event `enableMoveZ`
  ;[1 1 1] mouse Click Event --> C_MiniGame03
  (bind _isa (`/Engine/EditorBlueprintResources/StandardMacros.FlipFlop`)
    (:`A`
      _)
    (:`B`
      _))
  (set `self.moveZ` _isa))

(event `self.ReceiveBeginPlay`
  ;[1 1 1] start Events
  (`|ExecutionSequence`
    (:`then_0`
      (if true
        (`self.Set Start Speed X`)))))

(event `Set Start Speed X`
  (bind _charactermovement (`Character.CharacterMovement` (`GameplayStatics.GetPlayerCharacter` 0)))
  ;[1 1 1] set start speed X direction
  (set `CharacterMovementComponent.MaxWalkSpeed` (`CharacterMovementComponent.MaxWalkSpeed` _charactermovement) _charactermovement)
  (set `CharacterMovementComponent.MaxStepHeight` 0.0 _charactermovement))

(event `self.ReceiveTick`
  (params (DeltaSeconds :type "Float (single-precision)"))
  ;[1 1 1] start Events
  (set `self.delta` DeltaSeconds)
  (`|ExecutionSequence`
    (:`then_0`
      (if true
        (`self.Set Character Movement X`)))
    (:`then_1`
      (if false
        (`self.Set Character Movement Z mouse`)))
    (:`then_2`
      (if false
        (`self.Set Motion Step Z mouse`)))))

(event `Set Character Movement X`
  (bind _returnvalue (`GameplayStatics.GetPlayerCharacter` 0))
  (bind _returnvalue_2 (`GameplayStatics.GetPlayerCharacter` 0))
  (bind _charactermovement (`Character.CharacterMovement` _returnvalue))
  (bind _charactermovement_2 (`Character.CharacterMovement` _returnvalue_2))
  ;[1 1 1] set charakter movement x direction
  (if (`self.dialog`)
    _
    (elif (`self.boostState`)
      (`self.K2_SetActorLocation` _returnvalue_2 (`KismetMathLibrary.MakeVector` (+ (.x (`self.K2_GetActorLocation` _returnvalue_2)) (* (* (`CharacterMovementComponent.MaxWalkSpeed` _charactermovement_2) (`self.delta`)) (`self.boostSpeed`))) (.y (`self.K2_GetActorLocation` _returnvalue_2)) (+ (.z (`self.K2_GetActorLocation` _returnvalue_2)) (`CharacterMovementComponent.MaxStepHeight` _charactermovement_2))) false false)
      (else
        (`self.K2_SetActorLocation` _returnvalue (`KismetMathLibrary.MakeVector` (+ (.x (`self.K2_GetActorLocation` _returnvalue)) (* (`CharacterMovementComponent.MaxWalkSpeed` _charactermovement) (`self.delta`))) (.y (`self.K2_GetActorLocation` _returnvalue)) (+ (.z (`self.K2_GetActorLocation` _returnvalue)) (`CharacterMovementComponent.MaxStepHeight` _charactermovement))) false false)))))

(event `keyUp`
  (bind _motionstepz (`self.motionStepZ`))
  ;[1 1 1] set character movement with key up/down
  ;;[1 1 1] for BP_Partner
  (if (`self.dialog`)
    _
    (elif (< (`self.counterKeyMovement`) 2)
      (set `self.counterKeyMovement` (+ (`self.counterKeyMovement`) 1))
      (`self.K2_AddActorLocalOffset` (`GameplayStatics.GetPlayerCharacter` 0) (`KismetMathLibrary.MakeVector` 0.0 (/ _motionstepz -10.0) _motionstepz) false false))))

(event `Set Character Movement Z mouse`
  (bind _returnvalue (`self.K2_GetActorLocation` (`GameplayStatics.GetPlayerCharacter` 0)))
  (bind _charactermovement (`Character.CharacterMovement` (`GameplayStatics.GetPlayerCharacter` 0)))
  ;[1 1 1] set character movement z direction with mouse input
  (if (`self.moveZ`)
    (set `self.oldActorPosition` _returnvalue)
    (if (< (.z (`KismetMathLibrary.MakeVector` (.x (`.Location` (`GameplayStatics.BreakHitResult` (`PlayerController.GetHitResultUnderCursorByChannel` (`GameplayStatics.GetPlayerController` 0) "TraceTypeQuery1" true)))) (.y (`.Location` (`GameplayStatics.BreakHitResult` (`PlayerController.GetHitResultUnderCursorByChannel` (`GameplayStatics.GetPlayerController` 0) "TraceTypeQuery1" true)))) (.z (`.Location` (`GameplayStatics.BreakHitResult` (`PlayerController.GetHitResultUnderCursorByChannel` (`GameplayStatics.GetPlayerController` 0) "TraceTypeQuery1" true)))))) (.z _returnvalue))
      (set `CharacterMovementComponent.MaxStepHeight` -40.0 _charactermovement)
      (else
        (set `CharacterMovementComponent.MaxStepHeight` 40.0 _charactermovement)))))

(event `keyDown`
  (bind _motionstepz (`self.motionStepZ`))
  ;[1 1 1] set character movement with key up/down
  ;;[1 1 1] for BP_Partner
  (if (`self.dialog`)
    _
    (elif (> (`self.counterKeyMovement`) -2)
      (set `self.counterKeyMovement` (+ (`self.counterKeyMovement`) -1))
      (`self.K2_AddActorLocalOffset` (`GameplayStatics.GetPlayerCharacter` 0) (`KismetMathLibrary.MakeVector` 0.0 (/ _motionstepz 10.0) (* _motionstepz -1.0)) false false))))

(event `Set Motion Step Z mouse`
  (bind _motionstepz (`self.motionStepZ`))
  (bind _z (.z (`self.oldActorPosition`)))
  (bind _z_2 (.z (`self.K2_GetActorLocation` (`GameplayStatics.GetPlayerCharacter` 0))))
  ;[1 1 1] motion step Z direction
  (if (> (- _z _motionstepz) _z_2)
    (set `CharacterMovementComponent.MaxStepHeight` 0.0 (`Character.CharacterMovement` (`GameplayStatics.GetPlayerCharacter` 0)) :!label _label)
    (elif (< (+ _z _motionstepz) _z_2)
      (goto _label)
      (else
        (set `self.moveZ` false)))))

(event `Set Boost`
  ;[1 1 1] Use Boost
  (set `self.boostState` true)
  (`GameplayStatics.PlaySound2D` "/Game/Sounds/S_boost.S_Boost")
  (`KismetSystemLibrary.Delay` 1.0)
  (set `self.boostState` false))

(fn `UserConstructionScript`)