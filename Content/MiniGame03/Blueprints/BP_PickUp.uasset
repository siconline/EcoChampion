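; Wheelbarrow minigame pickup that plays a grow-and-shrink animation and destroys itself when a Character touches it.
; Overlap saves walk speed once via DoN, disables input and sets a Scale flag.
; Tick applies the indexed material and steps the animation with zero walk speed, restoring speed and input on destroy.
; Full and empty wheelbarrow events shift the pickup along Y and toggle its box collision, with a delay when full.
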(event `self.ReceiveBeginPlay`
  ;[1 1 1] start Events
  (`|ExecutionSequence`
    (:`then_0`
      (if true
        _))))

(event `Set Value for animation scale`
  (params (`Other Actor` :type "Actor Object Reference"))
  ;[1 1 1] set value for animation scale
  (cast `Character` `Other Actor`)
  (set `self.scale` true))

(event `full weelbarrow`
  ;[1 1 1] regulates behavior when weelbarrow full
  (`KismetSystemLibrary.Delay` 0.5)
  (`PrimitiveComponent.SetCollisionEnabled` (`self.Box`) "NoCollision")
  (`self.K2_SetActorLocation` (`KismetMathLibrary.MakeVector` (.x (`self.K2_GetActorLocation`)) -30.0 (.z (`self.K2_GetActorLocation`)))))

(event `Save MaxWalkSpeed`
  (params (`Other Actor` :type "Actor Object Reference"))
  ;[1 1 1] save MaxWalkSpeed and diable input
  (bind _ascharacter (cast `Character` `Other Actor`))
  (`/Engine/EditorBlueprintResources/StandardMacros.Do N` 1 :!label _label
    (:`Exit`
      (set `self.saveMaxWalkSpeed` (`CharacterMovementComponent.MaxWalkSpeed` (`Character.CharacterMovement` _ascharacter)))
      (`self.DisableInput` _ascharacter (`GameplayStatics.GetPlayerController` 0)))))

(event `reset`
  ;[1 1 1] save MaxWalkSpeed and diable input
  (`self.EnableInput` (`GameplayStatics.GetPlayerCharacter` 0) (`GameplayStatics.GetPlayerController` 0))
  (goto _label :!via `Reset`))

(event `self.ReceiveTick`
  (params (DeltaSeconds :type "Float (single-precision)"))
  ;[1 1 1] start Events
  (`|ExecutionSequence`
    (:`then_0`
      (if true
        (`self.Set Material PickUp`)))
    (:`then_1`
      (if true
        (`self.Play Animation Scale`)))))

(event `empty weelbarrow`
  ;[1 1 1] regulates behavior when weelbarrow full
  (`PrimitiveComponent.SetCollisionEnabled` (`self.Box`) "QueryAndPhysics")
  (`self.K2_SetActorLocation` (`KismetMathLibrary.MakeVector` (.x (`self.K2_GetActorLocation`)) 5.0 (.z (`self.K2_GetActorLocation`)))))

(event `Set Material PickUp`
  ;[1 1 1] set standard material
  (`PrimitiveComponent.SetMaterial` (`self.StaticMesh`) 0 (`|GetArrayItem` (`self.arrayMaterial`) (`self.index`))))

(event `self.ReceiveActorBeginOverlap`
  (params (OtherActor :type "Actor Object Reference"))
  ;[1 1 1] start Events
  (`|ExecutionSequence`
    (:`then_0`
      (if true
        (`self.Save MaxWalkSpeed` OtherActor)))
    (:`then_1`
      (if true
        (`self.Set Value for animation scale` OtherActor)))))

(event `Play Animation Scale`
  ;[1 1 1] set boolean SCALE --> true -- begin actor grow and shrink
  (if (`self.scale`)
    (set `CharacterMovementComponent.MaxWalkSpeed` 0.0 (`Character.CharacterMovement` (`GameplayStatics.GetPlayerCharacter` 0)))
    (if (>= (.x (`self.scaleValue`)) (`self.scaleFactor`))
      (set `self.scaleFactor` 0.0)
      (bind _output_get (set `self.scaleValue` (- (`self.scaleValue`) (0.2 0.2 0.0))))
      (`self.K2_AddActorLocalTransform` (`KismetMathLibrary.MakeTransform` (0.0 5.0 0.0) (struct) _output_get))
      (if (<= (.x (`self.scaleValue`)) 0.0)
        (`self.Destroy Actor`))
      (elif (not (<= (`self.scaleFactor`) 0.0))
        (bind _output_get_2 (set `self.scaleValue` (+ (`self.scaleValue`) (0.05 0.05 0.0))))
        (`self.K2_AddActorLocalTransform` (`KismetMathLibrary.MakeTransform` (0.0 5.0 0.0) (struct) _output_get_2))))))

(event `Destroy Actor`
  ;[1 1 1] destroy actor -- reset charactermovement speed -- reset boolean SCALE
  (`self.K2_DestroyActor`)
  (set `CharacterMovementComponent.MaxWalkSpeed` (`self.saveMaxWalkSpeed`) (`Character.CharacterMovement` (`GameplayStatics.GetPlayerCharacter` 0)))
  (set `self.scale` false)
  (`self.reset`))

(fn `UserConstructionScript`)