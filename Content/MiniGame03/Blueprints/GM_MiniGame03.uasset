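; Game mode for MiniGame03 that runs a countdown and ends the level when all pickups are gone or time runs out.
; Tick drives the minutes/seconds countdown, with a one-second Delay pacing it, and pauses to show the time-out widget at zero.
; Tick also polls for BP_PickUp and BP_PickUpMove actors; when none remain and no main menu exists, it waits briefly, shows that menu and opens MainLevel.
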(event `self.ReceiveTick`
  (params (DeltaSeconds :type "Float (single-precision)"))
  ;[1 1 1] start Events
  (`|ExecutionSequence`
    (:`then_0`
      (if true
        (`self.TimerCounter`)))
    (:`then_1`
      (bind _foundwidgets (`WidgetBlueprintLibrary.GetAllWidgetsOfClass` "/Game/Menu/Widget_MainMenu.Widget_MainMenu_C" false))
      (if (< (`KismetArrayLibrary.Array_LastIndex` _foundwidgets) 0)
        (bind _outactors (`GameplayStatics.GetAllActorsOfClass` "/Game/MiniGame03/Blueprints/BP_PickUp.BP_PickUp_C"))
        (if (< (`KismetArrayLibrary.Array_LastIndex` _outactors) 0)
          (bind _outactors_2 (`GameplayStatics.GetAllActorsOfClass` "/Game/MiniGame03/Blueprints/BP_PickUpMove.BP_PickUpMove_C"))
          (if (< (`KismetArrayLibrary.Array_LastIndex` _outactors_2) 0)
            (`KismetSystemLibrary.Delay` 1.9)
            (`WidgetLayoutLibrary.RemoveAllWidgets`)
            (bind _returnvalue (`|CreateWidget` "/Game/Menu/Widget_MainMenu.Widget_MainMenu_C"))
            (`UserWidget.AddToViewport` _returnvalue 0)
            (`GameplayStatics.OpenLevel` "MainLevel")))))))

(event `TimerCounter`
  ;[1 1 1] Timer für GameOver wenn Zeit abgelaufen ist
  (`KismetSystemLibrary.Delay` 1.0)
  (set `self.seconds` (- (`self.seconds`) 1))
  (if (< (`self.seconds`) 0)
    (set `self.minutes` (- (`self.minutes`) 1))
    (set `self.seconds` 59))
  (if (== (`self.seconds`) 0)
    (if (== (`self.minutes`) 0)
      (`KismetSystemLibrary.PrintString` "time out")
      (`GameplayStatics.SetGamePaused` true)
      ;[1 1 1] Läd Time Out Menu
      (`WidgetLayoutLibrary.RemoveAllWidgets`)
      (bind _returnvalue (`|CreateWidget` "/Game/Menu/Widget_TimeOut.Widget_TimeOut_C"))
      (`UserWidget.AddToViewport` _returnvalue 0))))

(fn `UserConstructionScript`)