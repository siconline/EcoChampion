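; BP_SpawnBackground builds the scrolling-level backdrop for MiniGame03 from a row of BP_BackgroundTile actors.
; On BeginPlay it loops from zero to LevelLength + 1, spawning each tile offset along X by its index times BackgroundWidth.
; Each tile's plane material depends on index: a start material first, M_Flower for the last, and the middle material for the LevelLength tiles between.
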(event `self.ReceiveBeginPlay`
  ;[1 1 1] Loop Level Length -> Level Length = number of "Middle" tiles.
  (for _index (range (+ (+ 1 (`self.levelLength`)) 1))
    ;[1 1 1] Spawns BP_BackgroundTiles and offsets them according to index times Background Width
    (bind _returnvalue (`|SpawnActorFromClass` "/Game/MiniGame03/Blueprints/BP_BackgroundTile.BP_BackgroundTile_C" (`KismetMathLibrary.Conv_VectorToTransform` (`KismetMathLibrary.MakeVector` (`KismetMathLibrary.Conv_IntToDouble` (* _index (`self.backgroundWidth`))))) "Undefined" "OverrideRootScale" null null))
    ;[1 1 1] Sets texture depending on index (0 = start, Level Length + 1 (Last Index) = end, everything else = middle)
    (if (== 0 _index)
      (bind _plane (`/Game/MiniGame03/Blueprints/BP_BackgroundTile.Plane` _returnvalue))
      (`PrimitiveComponent.SetMaterial` _plane 0 "/Game/Materials/M_BackgroundStart.M_BackgroundStart")
      (elif (== (+ 1 (`self.levelLength`)) _index)
        (`PrimitiveComponent.SetMaterial` _plane 0 "/Game/Materials/M_Flower.M_Flower")
        (else
          (`PrimitiveComponent.SetMaterial` _plane 0 "/Game/Materials/M_BackgroundMiddle.M_BackgroundMiddle"))))))

(fn `UserConstructionScript`)